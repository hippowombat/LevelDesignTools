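; Prototype construction-script generator that builds a building interior with outer walls, corner rooms, door openings and a floor from a grid-snapped control spline.
; Geometry Script triangulates and extrudes the outline, then boolean-subtracts an inset copy to hollow walls.
; Per-point corner sizes create temporary room splines that get the same treatment, and boxes aligned to the control spline cut doors.
; The result can be copied to a static mesh asset.
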(event EventBeginPlay)

(event Collision|EventActorBeginOverlap
  (params (OtherActor :type Actor%20Object%20Reference)))

(event EventTick
  (params (DeltaSeconds :type Float%20%28single-precision%29)))

(fn ConstructionScript
  (if (< (Spline|GetNumberOfSplinePoints (Variables|Default|GetControlSpline)) 3)
    (CallFunction|ResetSplinetoSquare)
    (else
      (CallFunction|GenerateInterior))))

(fn ResetSplinetoSquare
  (Spline|ClearSplinePoints (Variables|Default|GetControlSpline) false)
  (for _array_element (Utilities|Array|MakeArray "0.750000,-1.000000,0.000000" "-0.750000,-1.000000,0.000000" "-0.750000,1.000000,0.000000" "0.750000,1.000000,0.000000")
    (Spline|AddSplinePoint (Variables|Default|GetControlSpline) (* _array_element (Math|Float|MakeLiteralFloat 5e+02)) "Local" false))
  (Spline|UpdateSpline (Variables|Default|GetControlSpline))
  (CallFunction|GenerateInterior)
  (return))

(fn SetCornerSizeArrayLengthtoSplinePointCount
  (bind _controlspline (Variables|Default|GetControlSpline))
  (bind _returnvalue (Spline|GetNumberOfSplinePoints _controlspline))
  (if (!= (Utilities|Array|Length (Variables|Default|GetRoomCornerSizes)) _returnvalue)
    (Utilities|Array|Resize (Variables|Default|GetRoomCornerSizes) _returnvalue))
  (return))

(fn DrawCornerRoomWallSplinePoints
  (CallFunction|ClearTempSplines)
  (for (_array_element _array_index) (Variables|Default|GetRoomCornerSizes)
    (LocalVariables|SetCurrentRoomDimensions _array_element)
    (bind _output_get (LocalVariables|SetCurrentRoomIndex _array_index))
    (if (and (> (.X (Math|Vector2D|BreakVector2D _array_element)) 0.0) (> (.Y (Math|Vector2D|BreakVector2D _array_element)) 0.0))
      (LocalVariables|SetCurrentRoomPoints (CallFunction|GetRoomSplineCornerPoints _output_get (LocalVariables|GetCurrentRoomDimensions)))
      (bind _returnvalue (AddComponent|AddSplineComponent false))
      (Spline|ClearSplinePoints _returnvalue true)
      (Utilities|Array|Add (Variables|Default|GetRoomSplines) _returnvalue)
      (for (_array_element_2 _array_index_2) (LocalVariables|GetCurrentRoomPoints)
        (Spline|AddSplinePoint _returnvalue _array_element_2 "Local" true)
        (Spline|SetSplinePointType _returnvalue _array_index_2 "Constant" true))
      (Class|SplineComponent|SetUnselectedSplineSegmentColor _returnvalue (Utilities|Struct|MakeLinearColor 1.0 0.0 1.0 0.0))))
  (return))

(fn GetRoomSplineCornerPoints
  (params (PointIndex :type Integer) (Extents :type Vector%202D%20Structure%20%28by%20ref%29))
  (bind _controlspline (Variables|Default|GetControlSpline))
  (bind _returnvalue (Spline|GetLocationatSplinePoint _controlspline PointIndex "Local"))
  (LocalVariables|SetLastIndex (- (Spline|GetNumberOfSplinePoints (Variables|Default|GetControlSpline)) 1))
  (return (Utilities|Array|MakeArray _returnvalue (+ _returnvalue (* (Math|Vector|GetForwardVector (Math|Rotator|FindLookatRotation _returnvalue (Spline|GetLocationatSplinePoint (Variables|Default|GetControlSpline) (Math|Integer|SelectInt 0 (+ PointIndex 1) (== PointIndex (LocalVariables|GetLastIndex))) "Local"))) (.x Extents))) (+ _returnvalue (* (Math|Vector|GetForwardVector (Math|Rotator|FindLookatRotation _returnvalue (Spline|GetLocationatSplinePoint (Variables|Default|GetControlSpline) (Math|Integer|SelectInt 0 (+ PointIndex 1) (== PointIndex (LocalVariables|GetLastIndex))) "Local"))) (.x Extents)) (* (.y Extents) (Math|Vector|GetForwardVector (Math|Rotator|FindLookatRotation _returnvalue (Spline|GetLocationatSplinePoint (Variables|Default|GetControlSpline) (Math|Integer|SelectInt (LocalVariables|GetLastIndex) (- PointIndex 1) (== PointIndex 0)) "Local"))))) (+ _returnvalue (* (.y Extents) (Math|Vector|GetForwardVector (Math|Rotator|FindLookatRotation _returnvalue (Spline|GetLocationatSplinePoint (Variables|Default|GetControlSpline) (Math|Integer|SelectInt (LocalVariables|GetLastIndex) (- PointIndex 1) (== PointIndex 0)) "Local"))))))))

(fn SnapControlSplinetoGrid
  (bind _controlspline (Variables|Default|GetControlSpline))
  (bind _splinepointindex (Utilities|ForEachSplinePoint _controlspline)
    (:LoopBody
      (Spline|SetLocationatSplinePoint _controlspline _splinepointindex (Class|KismetMathLibrary|VectorSnappedtoGrid (Spline|GetLocationatSplinePoint _controlspline _splinepointindex "Local") (Variables|Default|GetGridSnapSize)) "Local" true))
    (:Completed
      (return))))

(fn DrawOuterWalls
  (bind _outerwallpoints (LocalVariables|GetOuterWallPoints))
  (bind _controlspline (Variables|Default|GetControlSpline))
  (bind _returnvalue (Utilities|Array|LastIndex _outerwallpoints))
  (bind _returnvalue_2 (Class|DynamicMeshActor|GetComputeMeshPool))
  (bind _returnvalue_3 (Class|DynamicMeshPool|RequestMesh _returnvalue_2))
  (LocalVariables|SetComputeMesh _returnvalue_3)
  (bind _splinepointindex (Utilities|ForEachSplinePoint (Variables|Default|GetControlSpline))
    (:LoopBody
      (Utilities|Array|Add (LocalVariables|GetSplinePoints) (Spline|GetLocationatSplinePoint (Variables|Default|GetControlSpline) _splinepointindex "Local")))
    (:Completed
      (LocalVariables|SetSplinePointsAverage (Math|Vector|GetVectorArrayAverage (LocalVariables|GetSplinePoints)))
      ;[1 1 1] OuterWalls Outside
      (bind _splinepointindex_2 (Utilities|ForEachSplinePoint (Variables|Default|GetControlSpline))
        (:LoopBody
          (Utilities|Array|Add (LocalVariables|GetOuterWallPoints) (Math|Conversions|ToVector2D(Vector) (Spline|GetLocationatSplinePoint _controlspline _splinepointindex_2 "Local")))
          (Utilities|Array|Add (LocalVariables|GetOuterWallConstraints) (Utilities|Struct|MakeIntPoint _splinepointindex_2 (Math|Integer|SelectInt 0 (+ _splinepointindex_2 1) (== (+ _splinepointindex_2 1) (Spline|GetNumberOfSplinePoints _controlspline))))))
        (:Completed
          (bind _returnvalue_4 (Class|GeometryScriptLibraryMeshPrimitiveFunctions|AppendDelaunayTriangulation2D :TargetMesh (LocalVariables|GetComputeMesh) :VertexPositions (LocalVariables|GetOuterWallPoints) :ConstrainedEdges (LocalVariables|GetOuterWallConstraints) :TriangulationOptions (Utilities|Struct|MakeGeometryScriptConstrainedDelaunayTriangulationOptions "NegativeWinding" false false) :Debug 0))
          (bind _returnvalue_5 (DynamicMeshComponent|GetDynamicMesh (Variables|DynamicMeshActor|GetDynamicMeshComponent)))
          (bind _returnvalue_6 (GeometryScript|MeshEdits|AppendMesh :TargetMesh _returnvalue_5 :AppendMesh _returnvalue_4 :AppendOptions "(CombineMode=EnableAllMatching)" :Debug 0))
          (Class|GeometryScriptLibraryMeshModelingFunctions|ApplyMeshLinearExtrudeFaces :TargetMesh _returnvalue_6 :Options (Utilities|Struct|MakeGeometryScriptMeshLinearExtrudeOptions (Variables|Default|GetWallsHeight) "FixedDirection") :Debug 0)
          (DynamicMesh|Reset (LocalVariables|GetComputeMesh))
          ;[1 1 1] Outer walls inside
          (for (_array_element _array_index) _outerwallpoints
            (Utilities|Array|Add (LocalVariables|GetInnerWallPoints) (+ _array_element (select (< (Math|Vector|DotProduct (Math|Vector|GetForwardVector (Math|Rotator|FindLookatRotation (Math|Conversions|ToVector(Vector2D) _array_element) (+ (Math|Conversions|ToVector(Vector2D) _array_element) (* (Math|Vector|GetVectorArrayAverage (Utilities|Array|MakeArray (Math|Vector|GetForwardVector (Math|Rotator|FindLookatRotation (Math|Conversions|ToVector(Vector2D) _array_element) (Math|Conversions|ToVector(Vector2D) (Utilities|Array|Get(acopy) _outerwallpoints (Math|Integer|SelectInt 0 (+ _array_index 1) (== _array_index _returnvalue)))))) (Math|Vector|GetForwardVector (Math|Rotator|FindLookatRotation (Math|Conversions|ToVector(Vector2D) _array_element) (Math|Conversions|ToVector(Vector2D) (Utilities|Array|Get(acopy) _outerwallpoints (Math|Integer|SelectInt _returnvalue (- _array_index 1) (== _array_index 0)))))))) (Variables|Default|GetWallsThickness))))) (Math|Vector|GetForwardVector (Math|Rotator|FindLookatRotation (Math|Conversions|ToVector(Vector2D) _array_element) (LocalVariables|GetSplinePointsAverage)))) 0.0) (* (Math|Conversions|ToVector2D(Vector) (* (Math|Vector|GetVectorArrayAverage (Utilities|Array|MakeArray (Math|Vector|GetForwardVector (Math|Rotator|FindLookatRotation (Math|Conversions|ToVector(Vector2D) _array_element) (Math|Conversions|ToVector(Vector2D) (Utilities|Array|Get(acopy) _outerwallpoints (Math|Integer|SelectInt 0 (+ _array_index 1) (== _array_index _returnvalue)))))) (Math|Vector|GetForwardVector (Math|Rotator|FindLookatRotation (Math|Conversions|ToVector(Vector2D) _array_element) (Math|Conversions|ToVector(Vector2D) (Utilities|Array|Get(acopy) _outerwallpoints (Math|Integer|SelectInt _returnvalue (- _array_index 1) (== _array_index 0)))))))) (Variables|Default|GetWallsThickness))) "(X=-1.000000,Y=-1.000000)") (Math|Conversions|ToVector2D(Vector) (* (Math|Vector|GetVectorArrayAverage (Utilities|Array|MakeArray (Math|Vector|GetForwardVector (Math|Rotator|FindLookatRotation (Math|Conversions|ToVector(Vector2D) _array_element) (Math|Conversions|ToVector(Vector2D) (Utilities|Array|Get(acopy) _outerwallpoints (Math|Integer|SelectInt 0 (+ _array_index 1) (== _array_index _returnvalue)))))) (Math|Vector|GetForwardVector (Math|Rotator|FindLookatRotation (Math|Conversions|ToVector(Vector2D) _array_element) (Math|Conversions|ToVector(Vector2D) (Utilities|Array|Get(acopy) _outerwallpoints (Math|Integer|SelectInt _returnvalue (- _array_index 1) (== _array_index 0)))))))) (Variables|Default|GetWallsThickness)))))))
          (bind _returnvalue_7 (Class|GeometryScriptLibraryMeshPrimitiveFunctions|AppendDelaunayTriangulation2D :TargetMesh (LocalVariables|GetComputeMesh) :Transform (Math|Conversions|ToTransform(Vector) (Math|Vector|MakeVector 0.0 0.0 -5e+01)) :VertexPositions (LocalVariables|GetInnerWallPoints) :ConstrainedEdges (LocalVariables|GetOuterWallConstraints) :TriangulationOptions (Utilities|Struct|MakeGeometryScriptConstrainedDelaunayTriangulationOptions "NegativeWinding" false false) :Debug 0))
          (bind _returnvalue_8 (Class|GeometryScriptLibraryMeshModelingFunctions|ApplyMeshLinearExtrudeFaces :TargetMesh _returnvalue_7 :Options (Utilities|Struct|MakeGeometryScriptMeshLinearExtrudeOptions (+ (Variables|Default|GetWallsHeight) 1e+02) "FixedDirection") :Debug 0))
          (bind _returnvalue_9 (DynamicMeshComponent|GetDynamicMesh (Variables|DynamicMeshActor|GetDynamicMeshComponent)))
          (GeometryScript|Booleans|ApplyMeshBoolean :TargetMesh _returnvalue_9 :ToolMesh _returnvalue_8 :Operation "Subtract" :Options (Utilities|Struct|MakeGeometryScriptMeshBooleanOptions false true 0.01) :Debug 0)
          (bind _returnvalue_10 (DynamicMesh|Reset (LocalVariables|GetComputeMesh)))
          (Class|DynamicMeshActor|ReleaseComputeMesh _returnvalue_10)
          (return))))))

(fn DrawInnerRoomWalls
  (bind _outerwallpoints (LocalVariables|GetOuterWallPoints))
  (bind _returnvalue (Utilities|Array|LastIndex _outerwallpoints))
  (bind _returnvalue_2 (Class|DynamicMeshActor|GetComputeMeshPool))
  (bind _returnvalue_3 (Class|DynamicMeshPool|RequestMesh _returnvalue_2))
  (LocalVariables|SetComputeMesh _returnvalue_3)
  (bind _returnvalue_4 (Class|DynamicMeshActor|GetComputeMeshPool))
  (bind _returnvalue_5 (Class|DynamicMeshPool|RequestMesh _returnvalue_4))
  (LocalVariables|SetSubMesh _returnvalue_5)
  (for _array_element (Variables|Default|GetRoomSplines)
    (LocalVariables|SetCurrentSpline _array_element)
    ;[1 1 1] OuterWalls Outside
    (bind _splinepointindex (Utilities|ForEachSplinePoint (LocalVariables|GetCurrentSpline))
      (:LoopBody
        (Utilities|Array|Add (LocalVariables|GetOuterWallPoints) (Math|Conversions|ToVector2D(Vector) (Spline|GetLocationatSplinePoint (LocalVariables|GetCurrentSpline) _splinepointindex "Local")))
        (Utilities|Array|Add (LocalVariables|GetOuterWallConstraints) (Utilities|Struct|MakeIntPoint _splinepointindex (Math|Integer|SelectInt 0 (+ _splinepointindex 1) (== (+ _splinepointindex 1) (Spline|GetNumberOfSplinePoints (LocalVariables|GetCurrentSpline)))))))
      (:Completed
        (bind _returnvalue_6 (Class|GeometryScriptLibraryMeshPrimitiveFunctions|AppendDelaunayTriangulation2D :TargetMesh (LocalVariables|GetComputeMesh) :VertexPositions (LocalVariables|GetOuterWallPoints) :ConstrainedEdges (LocalVariables|GetOuterWallConstraints) :TriangulationOptions (Utilities|Struct|MakeGeometryScriptConstrainedDelaunayTriangulationOptions "NegativeWinding" false false) :Debug 0))
        (bind _returnvalue_7 (Class|GeometryScriptLibraryMeshModelingFunctions|ApplyMeshLinearExtrudeFaces :TargetMesh _returnvalue_6 :Options (Utilities|Struct|MakeGeometryScriptMeshLinearExtrudeOptions (Variables|Default|GetWallsHeight) "FixedDirection") :Debug 0))
        (bind _returnvalue_8 (DynamicMeshComponent|GetDynamicMesh (Variables|DynamicMeshActor|GetDynamicMeshComponent)))
        (GeometryScript|MeshEdits|AppendMesh :TargetMesh _returnvalue_8 :AppendMesh _returnvalue_7 :AppendOptions "(CombineMode=EnableAllMatching)" :Debug 0)
        ;[1 1 1] Outer walls inside
        (for (_array_element_2 _array_index) _outerwallpoints
          (Utilities|Array|Add (LocalVariables|GetInnerWallPoints) (+ _array_element_2 (Math|Conversions|ToVector2D(Vector) (* (Math|Vector|GetVectorArrayAverage (Utilities|Array|MakeArray (Math|Vector|GetForwardVector (Math|Rotator|FindLookatRotation (Math|Conversions|ToVector(Vector2D) _array_element_2) (Math|Conversions|ToVector(Vector2D) (Utilities|Array|Get(acopy) _outerwallpoints (Math|Integer|SelectInt 0 (+ _array_index 1) (== _array_index _returnvalue)))))) (Math|Vector|GetForwardVector (Math|Rotator|FindLookatRotation (Math|Conversions|ToVector(Vector2D) _array_element_2) (Math|Conversions|ToVector(Vector2D) (Utilities|Array|Get(acopy) _outerwallpoints (Math|Integer|SelectInt _returnvalue (- _array_index 1) (== _array_index 0)))))))) (Variables|Default|GetWallsThickness))))))
        (bind _returnvalue_9 (Class|GeometryScriptLibraryMeshPrimitiveFunctions|AppendDelaunayTriangulation2D :TargetMesh (LocalVariables|GetSubMesh) :Transform (Math|Conversions|ToTransform(Vector) (Math|Vector|MakeVector 0.0 0.0 -5e+01)) :VertexPositions (LocalVariables|GetInnerWallPoints) :ConstrainedEdges (LocalVariables|GetOuterWallConstraints) :TriangulationOptions (Utilities|Struct|MakeGeometryScriptConstrainedDelaunayTriangulationOptions "NegativeWinding" false false) :Debug 0))
        (bind _returnvalue_10 (Class|GeometryScriptLibraryMeshModelingFunctions|ApplyMeshLinearExtrudeFaces :TargetMesh _returnvalue_9 :Options (Utilities|Struct|MakeGeometryScriptMeshLinearExtrudeOptions (+ (Variables|Default|GetWallsHeight) 1e+02) "FixedDirection") :Debug 0))
        (bind _returnvalue_11 (DynamicMeshComponent|GetDynamicMesh (Variables|DynamicMeshActor|GetDynamicMeshComponent)))
        (GeometryScript|Booleans|ApplyMeshBoolean :TargetMesh _returnvalue_11 :ToolMesh _returnvalue_10 :Operation "Subtract" :Options (Utilities|Struct|MakeGeometryScriptMeshBooleanOptions false true 0.01) :Debug 0)
        (DynamicMesh|Reset (LocalVariables|GetComputeMesh))
        (DynamicMesh|Reset (LocalVariables|GetSubMesh))
        (Utilities|Array|Clear (LocalVariables|GetOuterWallPoints))
        (Utilities|Array|Clear (LocalVariables|GetOuterWallConstraints))
        (Utilities|Array|Clear (LocalVariables|GetInnerWallPoints)))))
  (DynamicMeshActor|ReleaseAllComputeMeshes)
  (return))

(fn DrawFloor
  (bind _controlspline (Variables|Default|GetControlSpline))
  (bind _returnvalue (Class|DynamicMeshActor|GetComputeMeshPool))
  (bind _returnvalue_2 (Class|DynamicMeshPool|RequestMesh _returnvalue))
  (LocalVariables|SetComputeMesh _returnvalue_2)
  ;[1 1 1] OuterWalls Outside
  (bind _splinepointindex (Utilities|ForEachSplinePoint (Variables|Default|GetControlSpline))
    (:LoopBody
      (Utilities|Array|Add (LocalVariables|GetOuterWallPoints) (Math|Conversions|ToVector2D(Vector) (Spline|GetLocationatSplinePoint _controlspline _splinepointindex "Local")))
      (Utilities|Array|Add (LocalVariables|GetOuterWallConstraints) (Utilities|Struct|MakeIntPoint _splinepointindex (Math|Integer|SelectInt 0 (+ _splinepointindex 1) (== (+ _splinepointindex 1) (Spline|GetNumberOfSplinePoints _controlspline))))))
    (:Completed
      (bind _returnvalue_3 (Class|GeometryScriptLibraryMeshPrimitiveFunctions|AppendDelaunayTriangulation2D :TargetMesh (LocalVariables|GetComputeMesh) :Transform (Math|Conversions|ToTransform(Vector) (Math|Vector|MakeVector 0.0 0.0 1.0)) :VertexPositions (LocalVariables|GetOuterWallPoints) :ConstrainedEdges (LocalVariables|GetOuterWallConstraints) :TriangulationOptions (Utilities|Struct|MakeGeometryScriptConstrainedDelaunayTriangulationOptions "NegativeWinding" false false) :Debug 0))
      (bind _returnvalue_4 (DynamicMeshComponent|GetDynamicMesh (Variables|DynamicMeshActor|GetDynamicMeshComponent)))
      (GeometryScript|MeshEdits|AppendMesh :TargetMesh _returnvalue_4 :AppendMesh _returnvalue_3 :AppendOptions "(CombineMode=EnableAllMatching)" :Debug 0)
      (DynamicMeshActor|ReleaseAllComputeMeshes)
      (return))))

(fn ClearTempSplines
  (bind _arrayelement (Utilities|Array|ReverseforEachLoop (Variables|Default|GetRoomSplines))
    (:LoopBody
      (Components|DestroyComponent _arrayelement))
    (:Completed
      (Utilities|Array|Clear (Variables|Default|GetRoomSplines))
      (return))))

(fn PunchDoors
  (bind _doorscale (Variables|Default|GetDoorScale))
  (bind _returnvalue (Class|DynamicMeshActor|GetComputeMeshPool))
  (bind _returnvalue_2 (Class|DynamicMeshPool|RequestMesh _returnvalue))
  (LocalVariables|SetComputeMesh _returnvalue_2)
  (for (_array_element _array_index) (Variables|Default|GetDoorPositions)
    (Utilities|Array|SetArrayElem (Variables|Default|GetDoorPositions) _array_index (* _array_element "1.000000,1.000000,0.000000"))
    (bind _output_get (LocalVariables|SetCurrentDoorPosition (* _array_element "1.000000,1.000000,0.000000")))
    (bind _returnvalue_3 (DynamicMesh|Reset (LocalVariables|GetComputeMesh)))
    (bind _returnvalue_4 (Class|GeometryScriptLibraryMeshPrimitiveFunctions|AppendBox :TargetMesh _returnvalue_3 :Transform (Math|Transform|MakeTransform (LocalVariables|GetCurrentDoorPosition) (Math|Conversions|RotationFromXVector (Class|SplineComponent|FindTangentClosesttoWorldLocation (Variables|Default|GetControlSpline) (Math|Transform|TransformLocation (Transformation|GetActorTransform) _output_get) "World")) "1.000000,1.000000,1.000000") :DimensionX (.x _doorscale) :DimensionY (.y _doorscale) :DimensionZ (.z _doorscale) :Debug 0))
    (bind _returnvalue_5 (DynamicMeshComponent|GetDynamicMesh (Variables|DynamicMeshActor|GetDynamicMeshComponent)))
    (GeometryScript|Booleans|ApplyMeshBoolean :TargetMesh _returnvalue_5 :ToolMesh _returnvalue_4 :Operation "Subtract" :Debug 0))
  (DynamicMeshActor|ReleaseAllComputeMeshes)
  (return))

(fn SetAllSplinePointstoSpecifiedType
  (bind _controlspline (Variables|Default|GetControlSpline))
  (bind _splinepointindex (Utilities|ForEachSplinePoint _controlspline)
    (:LoopBody
      (Spline|SetSplinePointType _controlspline _splinepointindex "Linear" false))
    (:Completed
      (return))))

(fn LabelControlSplinePointIndices
  (bind _controlspline (Variables|Default|GetControlSpline))
  (bind _textrendercomps (Variables|Default|GetTextRenderComps))
  (bind _arrayelement (Utilities|Array|ReverseforEachLoop _textrendercomps)
    (:LoopBody
      (Components|DestroyComponent _arrayelement))
    (:Completed
      (Utilities|Array|Clear _textrendercomps)
      (bind _splinepointindex (Utilities|ForEachSplinePoint _controlspline)
        (:LoopBody
          (bind _returnvalue (AddComponent|AddTextRenderComponent false (Math|Transform|MakeTransform (+ (Spline|GetLocationatSplinePoint _controlspline _splinepointindex "Local") (Math|Vector|MakeVector 0.0 0.0 5e+01)) "0.000000,180.000000,0.000000" "1.000000,1.000000,1.000000")))
          (Utilities|Array|Add (Variables|Default|GetTextRenderComps) _returnvalue)
          (Rendering|Components|TextRender|SetText _returnvalue (Utilities|Text|ToText(String) (Utilities|String|ToString(Integer) _splinepointindex))))
        (:Completed
          (return))))))

(fn ConverttoStaticMesh
  (Variables|Default|GetStaticMeshAssetSaveTarget
    (:then
      (bind _returnvalue (DynamicMeshComponent|GetDynamicMesh (Variables|DynamicMeshActor|GetDynamicMeshComponent)))
      (GeometryScript|StaticMesh|CopyMeshtoStaticMesh :FromDynamicMesh _returnvalue :ToStaticMeshAsset (Variables|Default|GetStaticMeshAssetSaveTarget) :Debug 0
        (:Failure
          (Development|PrintString "Failed to write room to static mesh asset"))
        (:Success
          (Development|PrintString "Successfully wrote room to static mesh asset. Don't forget to save the asset!")))
      (return))
    (:else
      (Development|PrintString "Please set a value to StaticMeshAssetSaveTarget before converting to static mesh!" true true "(R=1.000000,G=0.250000,B=0.000000,A=1.000000)")
      (return))))

(fn GenerateInterior
  (bind _returnvalue (DynamicMeshComponent|GetDynamicMesh (Variables|DynamicMeshActor|GetDynamicMeshComponent)))
  (DynamicMesh|Reset _returnvalue)
  (CallFunction|LabelControlSplinePointIndices)
  (CallFunction|SetAllSplinePointstoSpecifiedType)
  (CallFunction|SnapControlSplinetoGrid)
  (CallFunction|SetCornerSizeArrayLengthtoSplinePointCount)
  (CallFunction|DrawCornerRoomWallSplinePoints)
  (CallFunction|DrawOuterWalls)
  (CallFunction|DrawInnerRoomWalls)
  (CallFunction|PunchDoors)
  (CallFunction|DrawFloor)
  (CallFunction|ClearTempSplines)
  (CallFunction|UpdateCollisions)
  (return))

(fn UpdateCollisions
  (Class|DynamicMeshComponent|UpdateCollision (Variables|DynamicMeshActor|GetDynamicMeshComponent) false)
  (return))